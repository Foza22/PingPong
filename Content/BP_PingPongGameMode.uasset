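; Game mode for a ping pong game that gives each joining player a separate start point.
; ChoosePlayerStart returns the first BasePlayerStart not tagged "Taken" and tags it so later players skip it.
; NewFunction is a debug check that prints whether a BasePlayerController has a valid pawn, with an unreachable PlayerPlatform cast left behind.
; BeginPlay, Tick and the construction script are empty.
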(event EventBeginPlay)

(event EventTick
  (params (DeltaSeconds :type Float%20%28single-precision%29)))

(fn ConstructionScript)

(fn ChoosePlayerStart
  (params (Player :type Controller%20Object%20Reference))
  (bind _outactors (Actor|GetAllActorsOfClass "/Script/PingPong.BasePlayerStart"))
  (for _array_element _outactors
    (if (!= (Variables|/Script/Engine.PlayerStart|GetPlayerStartTag _array_element) "Taken")
      (Variables|/Script/Engine.PlayerStart|SetPlayerStartTag _array_element "Taken")
      (return _array_element))))

(fn NewFunction
  (params (self2 :type Controller%20Object%20Reference))
  (bind _asbase_player_controller (Utilities|Casting|CastToBasePlayerController self2))
  (if (Utilities|IsValid (Pawn|GetControlledPawn _asbase_player_controller))
    (Development|PrintString "Hello")
    (else
      (Development|PrintString "Bye"))))